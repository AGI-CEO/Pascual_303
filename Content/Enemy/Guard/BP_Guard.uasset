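; BP_Guard is a patrolling enemy guard that catches the player on contact.
; From BeginPlay it uses AI MoveTo to walk between two patrol targets, pausing briefly at each before flipping a flag and recursively calling MoveToNextPoint.
; When its Box trigger overlaps BP_PlayerChar, it prints a caught message, waits, then reloads Level1 by name.
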(event `self.ReceiveBeginPlay`
  (`self.MoveToNextPoint`))

(event `MoveToNextPoint`
  (if (`self.bIsGoingToTarget1`)
    (`|AIMoveTo` self (0.0 0.0 0.0) (`self.PatrolTarget1`)
      (:`OnSuccess`
        (`KismetSystemLibrary.Delay` 3.0)
        (set `self.bIsGoingToTarget1` false)
        (`self.MoveToNextPoint`)))
    (else
      (`|AIMoveTo` self (0.0 0.0 0.0) (`self.PatrolTarget2`)
        (:`OnSuccess`
          (`KismetSystemLibrary.Delay` 3.0)
          (set `self.bIsGoingToTarget1` true)
          (`self.MoveToNextPoint`))))))

(event `self.Box.OnComponentBeginOverlap`
  (params (OverlappedComponent :type "PrimitiveComponent Object Reference") (OtherActor :type "Actor Object Reference") (OtherComp :type "PrimitiveComponent Object Reference") (OtherBodyIndex :type Integer) (bFromSweep :type Boolean) (SweepResult :type "HitResult Structure (by ref)"))
  (cast `/Game/Player/BP_PlayerChar` OtherActor)
  (`KismetSystemLibrary.PrintString` "Caught by GUARD!" true true (struct :`R` 1.0 :`B` 0.010602 :`A` 1.0) 3.0)
  (`KismetSystemLibrary.Delay` 2.2)
  (`GameplayStatics.OpenLevel` "Level1"))

(fn `UserConstructionScript`)